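; Anim notify state that shows a weapon trail effect on a BP_ky_bigSword actor for the notify's duration in an animation.
; On begin, it casts the mesh owner to the sword and starts trails on its PSCompo particle component between the trailStart and trailEnd sockets, with width measured from centre.
; On end, it ends those trails; other owner types are ignored.
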(fn ReceivedNotifyBegin
  (params (MeshComp :type Skeletal%20Mesh%20Component%20Object%20Reference) (Animation :type Anim%20Sequence%20Base%20Object%20Reference) (TotalDuration :type Float%20%28single-precision%29))
  ;[1 1 1] set trail FX
  (bind _asbp_ky_big_sword (Utilities|Casting|CastToBP_ky_bigSword (Components|GetOwner MeshComp)))
  (Effects|Particles|Trails|BeginTrails (Variables|/Game/AttackTrailFX01/Blueprints/BP_ky_bigSword.BP_ky_bigSword_C|GetPS_compo _asbp_ky_big_sword) "trailStart" "trailEnd" "ETrailWidthMode_FromCentre" 1.0)
  (return false))

(fn ReceivedNotifyEnd
  (params (MeshComp :type Skeletal%20Mesh%20Component%20Object%20Reference) (Animation :type Anim%20Sequence%20Base%20Object%20Reference))
  ;[1 1 1] trail FX finish
  (bind _asbp_ky_big_sword (Utilities|Casting|CastToBP_ky_bigSword (Components|GetOwner MeshComp)))
  (Effects|Particles|Trails|EndTrails (Variables|/Game/AttackTrailFX01/Blueprints/BP_ky_bigSword.BP_ky_bigSword_C|GetPS_compo _asbp_ky_big_sword))
  (return false))