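; BP_TestPlatform_Animations is a cube-based actor, named as an animation test platform, that gives itself a randomized look.
; Its Construction Script creates a dynamic instance of M_Basic on the Cube, stores it in CustomMaterial, then randomizes metallic, specular, roughness, emissive and base color.
; The values re-roll whenever construction runs, and the Event Graph holds only disabled placeholder events, with no animation or gameplay logic.
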(event EventBeginPlay)

(event Collision|EventActorBeginOverlap
  (params (OtherActor :type Actor%20Object%20Reference)))

(event EventTick
  (params (DeltaSeconds :type Float%20%28single-precision%29)))

(fn ConstructionScript
  (bind _returnvalue (Rendering|Material|CreateDynamicMaterialInstance (Variables|Default|GetCube) 0 "/Game/Revenant/_MaterialLibrary/M_Basic.M_Basic" "None" :!class /Script/Engine.PrimitiveComponent))
  (Variables|Default|SetCustom%20Material _returnvalue)
  (Utilities|FlowControl|Sequence
    (:then_0
      (Rendering|Material|SetScalarParameterValue (Variables|Default|GetCustom%20Material) "Metallic" (Math|Random|RandomFloat) :!class /Script/Engine.MaterialInstanceDynamic))
    (:then_1
      (Rendering|Material|SetScalarParameterValue (Variables|Default|GetCustom%20Material) "Specular" (Math|Random|RandomFloatinRange 1.0 5.0) :!class /Script/Engine.MaterialInstanceDynamic))
    (:then_2
      (Rendering|Material|SetScalarParameterValue (Variables|Default|GetCustom%20Material) "Roughness" (Math|Random|RandomFloat) :!class /Script/Engine.MaterialInstanceDynamic))
    (:then_3
      (Rendering|Material|SetScalarParameterValue (Variables|Default|GetCustom%20Material) "Emissive" (Math|Random|RandomFloat) :!class /Script/Engine.MaterialInstanceDynamic))
    (:then_4
      (Rendering|Material|SetVectorParameterValue (Variables|Default|GetCustom%20Material) "Base Color" (Utilities|Struct|MakeLinearColor (Math|Random|RandomFloat) (Math|Random|RandomFloat) (Math|Random|RandomFloat) 1.0) :!class /Script/Engine.MaterialInstanceDynamic))))