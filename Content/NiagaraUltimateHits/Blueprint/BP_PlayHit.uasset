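; Blueprint that repeatedly plays a Niagara hit effect on a skeletal mesh, apparently as a preview for the NiagaraUltimateHits effects.
; BeginPlay starts a looping timer on LOOP, which spawns the configured system at the configured scale each tick of that timer.
; The Skeletal flag selects either the configurable HitSocket with fully random rotation, or the hardcoded EyeFlare socket with a fixed rotation.
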(event Custom|LOOP
  (bind _returnvalue (Math|Random|RandomFloatinRange 0.0 3.6e+02))
  (bind _niagarap (Variables|Default|GetNiagaraP))
  (bind _scale (Variables|Default|GetScale))
  (if (Variables|Default|GetSkeletal)
    (Niagara|SpawnSystematLocation _niagarap (Transformation|GetSocketLocation (Variables|Default|GetSkeletalMesh) (Variables|Default|GetHitSocket)) (Math|Rotator|MakeRotator _returnvalue _returnvalue _returnvalue) (Math|Vector|MakeVector _scale _scale _scale))
    (else
      (Niagara|SpawnSystematLocation _niagarap (Transformation|GetSocketLocation (Variables|Default|GetSkeletalMesh) "EyeFlare") "0.0,90.000000,0.0" (Math|Conversions|ToVector(Float) (Variables|Default|GetScale))))))

(event EventBeginPlay
  (Utilities|Time|SetTimerbyFunctionName 0 "LOOP" (Variables|Default|GetTime) true))

(fn ConstructionScript)