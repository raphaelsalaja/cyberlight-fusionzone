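; Test sphere actor that gives itself a randomised look and re-randomises it about every five seconds.
; The Construction Script creates a dynamic instance of M_Basic with random surface, emissive and colour parameters.
; Tick runs through a Delay into RandomColour, which rerolls them but pins Specular and Intensity to constants.
; Colour interpolation starts from fresh random values each call, so changes jump rather than blend.
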(event EventBeginPlay)

(event Collision|EventActorBeginOverlap
  (params (OtherActor :type Actor%20Object%20Reference)))

(event EventTick
  (params (DeltaSeconds :type Float%20%28single-precision%29))
  (Utilities|FlowControl|Delay 5.0)
  (CallFunction|RandomColour))

(fn ConstructionScript
  (bind _returnvalue (Rendering|Material|CreateDynamicMaterialInstance (Variables|Default|GetSphere) 0 "/Game/Revenant/_MaterialLibrary/M_Basic.M_Basic" "None" :!class /Script/Engine.PrimitiveComponent))
  (Variables|Default|SetCustom%20Material _returnvalue)
  (Utilities|FlowControl|Sequence
    (:then_0
      (Rendering|Material|SetScalarParameterValue (Variables|Default|GetCustom%20Material) "Metallic" (Math|Random|RandomFloat) :!class /Script/Engine.MaterialInstanceDynamic))
    (:then_1
      (Rendering|Material|SetScalarParameterValue (Variables|Default|GetCustom%20Material) "Specular" (Math|Random|RandomFloatinRange 1.0 5.0) :!class /Script/Engine.MaterialInstanceDynamic))
    (:then_2
      (Rendering|Material|SetScalarParameterValue (Variables|Default|GetCustom%20Material) "Roughness" (Math|Random|RandomFloat) :!class /Script/Engine.MaterialInstanceDynamic))
    (:then_3
      (Rendering|Material|SetScalarParameterValue (Variables|Default|GetCustom%20Material) "Emissive" (Math|Random|RandomFloat) :!class /Script/Engine.MaterialInstanceDynamic))
    (:then_4
      (Rendering|Material|SetScalarParameterValue (Variables|Default|GetCustom%20Material) "Intensity" (Math|Random|RandomFloatinRange 2.0 5.0) :!class /Script/Engine.MaterialInstanceDynamic))
    (:then_5
      (Rendering|Material|SetVectorParameterValue (Variables|Default|GetCustom%20Material) "Base Color" (Class|KismetMathLibrary|CInterpto (Utilities|Struct|MakeLinearColor (CallFunction|IneterploateFloat 0.1) (CallFunction|IneterploateFloat 0.1) (CallFunction|IneterploateFloat 0.1) 1.0) (Utilities|Struct|MakeLinearColor (CallFunction|IneterploateFloat 0.1) (CallFunction|IneterploateFloat 0.1) (CallFunction|IneterploateFloat 0.1) 1.0) (Utilities|Time|GetWorldDeltaSeconds) 0.01) :!class /Script/Engine.MaterialInstanceDynamic))))

(fn RandomColour
  (bind _custom_material (Variables|Default|GetCustom%20Material))
  (Utilities|FlowControl|Sequence
    (:then_0
      (Rendering|Material|SetScalarParameterValue _custom_material "Metallic" (Math|Random|RandomFloat) :!class /Script/Engine.MaterialInstanceDynamic))
    (:then_1
      (Rendering|Material|SetScalarParameterValue _custom_material "Specular" (Math|Random|RandomFloatinRange 1.0 1.0) :!class /Script/Engine.MaterialInstanceDynamic))
    (:then_2
      (Rendering|Material|SetScalarParameterValue _custom_material "Roughness" (Math|Random|RandomFloat) :!class /Script/Engine.MaterialInstanceDynamic))
    (:then_3
      (Rendering|Material|SetScalarParameterValue _custom_material "Emissive" (Math|Random|RandomFloat) :!class /Script/Engine.MaterialInstanceDynamic))
    (:then_4
      (Rendering|Material|SetScalarParameterValue _custom_material "Intensity" (Math|Random|RandomFloatinRange 0.0 0.0) :!class /Script/Engine.MaterialInstanceDynamic))
    (:then_5
      (Rendering|Material|SetVectorParameterValue _custom_material "Base Color" (Class|KismetMathLibrary|CInterpto (Utilities|Struct|MakeLinearColor (CallFunction|IneterploateFloat 0.1) (CallFunction|IneterploateFloat 0.1) (CallFunction|IneterploateFloat 0.1) 1.0) (Utilities|Struct|MakeLinearColor (CallFunction|IneterploateFloat 0.1) (CallFunction|IneterploateFloat 0.1) (CallFunction|IneterploateFloat 0.1) 1.0) (Utilities|Time|GetWorldDeltaSeconds) 0.01) :!class /Script/Engine.MaterialInstanceDynamic))))

(fn IneterploateFloat
  (params (InterpSpeed :type Float%20%28double-precision%29))
  (return (Math|Interpolation|FInterpTo (Math|Random|RandomFloat) (Math|Random|RandomFloat) (Utilities|Time|GetWorldDeltaSeconds) InterpSpeed)))