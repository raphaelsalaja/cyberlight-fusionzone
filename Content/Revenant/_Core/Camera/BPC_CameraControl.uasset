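; Camera control component that drives a combat camera to keep all actors tagged "Actor" framed on screen.
; Each combat update glides a target toward the group's deprojected screen-box center, then orbits around it from look input with pitch compensation.
; Zoom interpolates distance by how far the focus box sits outside or inside a threshold box.
; The working transform passes through each step before being applied to the camera.
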(event Custom|Update%20Camera%20Combat%20Transform
  (Utilities|FlowControl|Sequence
    (:then_0
      (Variables|Default|SetNextFrameTransform (Transformation|GetActorTransform (Variables|Default|GetPlayer%20Camera)))
      (bind _outactors (Actor|GetAllActorswithTag "Actor"))
      (Variables|Default|SetActorsToFocus _outactors)
      (CallFunction|UpdateScreenInfo)
      (|MoveTarget_2_2)
      (|ApplyCameraInputRotation_2_2)
      (CallFunction|HandlePitchCompensation)
      (CallFunction|SetCameraFrameZoom))
    (:then_1
      (Transformation|SetActorTransform (Variables|Default|GetPlayer%20Camera) (Variables|Default|GetNextFrameTransform) false true))))

(event EventBeginPlay)

(event EventTick
  (params (DeltaSeconds :type Float%20%28single-precision%29)))

(fn UpdateScreenInfo)

(fn TransformSetLocation
  (params (Transform :type Transform) (Location :type Vector))
  (return ""))

(fn SetCameraFrameZoom
  (bind _cameratarget (Variables|Default|GetCameraTarget))
  (bind _focus_screen_box (Variables|Default|GetFocus%20Screen%20Box))
  (bind _zoomoutthresholdscreenbox (Variables|Default|GetZoomOutThresholdScreenBox))
  (bind _returnvalue (Transformation|GetActorLocation _cameratarget))
  (bind (_x _y) (Math|Vector2D|BreakVector2D (.max _focus_screen_box)))
  (bind (_x_2 _y_2) (Math|Vector2D|BreakVector2D (.max _zoomoutthresholdscreenbox)))
  (bind (_x_3 _y_3) (Math|Vector2D|BreakVector2D (.min _focus_screen_box)))
  (bind (_x_4 _y_4) (Math|Vector2D|BreakVector2D (.min _zoomoutthresholdscreenbox)))
  (Variables|Default|SetNextFrameTransform (Class|KismetMathLibrary|TInterpto (Variables|Default|GetNextFrameTransform) (CallFunction|TransformSetLocation (Variables|Default|GetNextFrameTransform) (+ (* (* (Math|Vector|GetForwardVector (.rotation (Variables|Default|GetNextFrameTransform))) -1.0) (* (Math|Float|Clamp(Float) (+ (/ (Math|Float|Max(Float) (- _x_4 _x_3) (- _y_4 _y_3) (- _x _x_2) (- _y _y_2)) (.y (Viewport|GetViewportSize))) 1.0) -1e+01 1e+01) (Math|Vector|Distance(Vector) _returnvalue (.location (Variables|Default|GetNextFrameTransform))))) _returnvalue)) (Utilities|Time|GetWorldDeltaSeconds) 5.0)))

(fn ApplyInputCameraRotation
  (params (Rotation :type Vector) (InitialTransform :type Transform%20%28by%20ref%29) (PivotLocation :type Vector) (Speed :type Float%20%28double-precision%29))
  (return ""))

(fn TransformSetRotation
  (params (Transform :type Transform) (Rotation :type Rotator))
  (return ""))

(fn HandlePitchCompensation
  (Variables|Default|SetNextFrameTransform (CallFunction|TransformSetRotation (CallFunction|TransformSetLocation (Variables|Default|GetNextFrameTransform) (CallFunction|ApplyInputCameraRotation (Math|Vector|MakeVector 0.0 (+ (Math|Vector|DotProduct (Transformation|GetActorForwardVector (Variables|Default|GetPlayer%20Camera)) "0,0.000000,1.000000") 0.5) 0.0) (Variables|Default|GetNextFrameTransform) (Transformation|GetActorLocation (Variables|Default|GetCameraTarget)) 1e+02)) (Math|Rotator|FindLookatRotation (.location (Variables|Default|GetNextFrameTransform)) (Transformation|GetActorLocation (Variables|Default|GetCameraTarget))))))