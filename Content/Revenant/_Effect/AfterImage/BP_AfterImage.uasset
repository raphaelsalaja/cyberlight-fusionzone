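; Afterimage actor that leaves a tinted, fading snapshot of a character's pose.
; SpawnAfterImage copies the pose from ModelReference onto a PoseableMesh and applies one dynamic instance of M_Mannequin_Afterimage to its material slots.
; A timeline drives that material's opacity alongside a hardcoded reddish BaseColor, then the actor destroys itself when the timeline finishes.
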(event Custom|Spawn%20After%20Image
  (params (Colour :type Linear%20Color%20Structure))
  (Variables|Default|SetColour "(R=0.510417,G=0.177937,B=0.114312,A=1.000000)")
  (bind _returnvalue (Rendering|Material|CreateDynamicMaterialInstance "/Game/AdvancedLocomotionV4/CharacterAssets/MannequinSkeleton/Materials/M_Mannequin_Afterimage.M_Mannequin_Afterimage" "None" "None" :!class /Script/Engine.KismetMaterialLibrary))
  (Variables|Default|SetAfterimage%20Material _returnvalue)
  (for _index (range 0 (Rendering|Material|GetNumMaterials (Variables|Default|GetModel%20Reference)))
    (Rendering|Material|SetMaterial (Variables|Default|GetPoseableMesh) _index (Variables|Default|GetAfterimage%20Material)))
  (Class|PoseableMeshComponent|CopyPosefromSkeletalComponent (Variables|Default|GetPoseableMesh) (Variables|Default|GetModel%20Reference))
  (bind _opacity (Timeline|Afterimage%20Timeline PlayFromStart)
    (:Update
      (Rendering|Material|SetVectorParameterValue (Variables|Default|GetAfterimage%20Material) "BaseColor" (Variables|Default|GetColour) :!class /Script/Engine.MaterialInstanceDynamic)
      (Rendering|Material|SetScalarParameterValue (Variables|Default|GetAfterimage%20Material) "Opacity" _opacity :!class /Script/Engine.MaterialInstanceDynamic))
    (:Finished
      (Actor|DestroyActor))))

(event EventBeginPlay)

(fn ConstructionScript)