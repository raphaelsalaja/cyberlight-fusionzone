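; BP_Player is a player character Blueprint with scaffolding for camera-relative target selection and switching, mostly unimplemented.
; GetActorAtDOT loops over candidate actors, scoring against the player camera's dot product, but its comparisons are unwired, so only the first actor gets picked.
; Target tracing, switching and construction are empty stubs.
; Movement checks, anim instance lookup and control-yaw direction graphs hold no connected logic.
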(fn ConstructionScript)

(fn TraceforTargets)

(fn GetActoratDOT
  (params (Distance :type Byte :default 0) (Actors :type Array%20of%20Actor%20Object%20References))
  (for (_array_element _array_index) Actors
    (if (== _array_index 0)
      (LocalVariables|SetDOT (Class|Actor|GetDotProductto (Game|GetPlayerCameraManager 0) _array_element) :!label _label)
      (LocalVariables|SetDOTActor _array_element)
      (elif (Utilities|Select :Index Distance :Option%200 false :Option%201 false)
        (goto _label))))
  (return (LocalVariables|GetDOTActor)))

(fn TargetSwitch
  (params (Left%20Or%20Right :type Byte :default 0)))