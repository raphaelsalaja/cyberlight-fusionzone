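; BP_EnemyTest is a child enemy character Blueprint that can be assigned to a team, including the player's.
; Its construction script runs the parent's, then copies Team into BPCombatComponent.
; On the player's team, it swaps the first two mesh materials to matte green and sets the text render to "Friendly".
; The event graph holds only disabled placeholder events, so it adds no runtime logic of its own.
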(event Collision|EventActorBeginOverlap
  (params (OtherActor :type Actor%20Object%20Reference))
  (|CallParentFunction OtherActor) ; This node is disabled and will not be called.\nDrag off pins to build functionality.
)

(event EventTick
  (params (DeltaSeconds :type Float%20%28single-precision%29))
  (|CallParentFunction DeltaSeconds) ; This node is disabled and will not be called.\nDrag off pins to build functionality.
)

(fn ConstructionScript
  (|CallParentFunction)
  (bind _output_get (Variables|/Game/Blueprints/Components/BP_CombatComponent.BP_CombatComponent_C|SetTeam (Variables|Default|GetBP_CombatComponent) (Variables|Default|GetTeam)))
  (if (== _output_get 0)
    (for _index (range 0 1)
      (Rendering|Material|SetMaterial (Variables|Character|GetMesh) _index "/Game/Blueprints/Characters/Enemy/ChildBlueprints/M_GreenMatte.M_GreenMatte"))
    (Rendering|Components|TextRender|SetText (Variables|Default|GetTextRender) (Utilities|Text|MakeLiteralText "Friendly"))))