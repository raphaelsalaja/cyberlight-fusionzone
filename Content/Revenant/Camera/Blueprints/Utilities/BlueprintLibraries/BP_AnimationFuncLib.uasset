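; Blueprint function library with a helper that supplies the basic movement variables an Animation Blueprint uses.
; GetDefaultAnimBPVariables takes an AnimInstance and, if its pawn owner is valid, returns whether the pawn is falling, its speed and its movement direction.
; Speed is the velocity's length, and direction comes from CalculateDirection using that velocity and the actor's rotation.
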(fn GetDefaultAnimBPVariables
  (params (Anim%20Instance :type Anim%20Instance%20Object%20Reference))
  (bind _returnvalue (Class|AnimInstance|TryGetPawnOwner Anim%20Instance))
  (bind _returnvalue_2 (Transformation|GetVelocity _returnvalue))
  (Utilities|IsValid _returnvalue
    (:Is%20Valid
      (return (AI|Components|NavMovement|IsFalling (Pawn|GetMovementComponent _returnvalue)) (Math|Vector|VectorLength _returnvalue_2) (Class|AnimInstance|CalculateDirection Anim%20Instance _returnvalue_2 (Transformation|GetActorRotation _returnvalue))))))