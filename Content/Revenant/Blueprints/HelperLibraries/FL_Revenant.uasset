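; Blueprint function library of shared gameplay helpers for Revenant, covering traces, vector math, capsule placement, array checks and gameplay tags.
; The cone trace fans sphere object traces in yaw around a forward vector, driven by a settings struct, and collects unique hit actors.
; Other helpers offset locations to capsule top or bottom and measure angles between vectors.
; Impure and pure tag checks fetch interface-provided tags and require exact matches of all requested tags.
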(fn ConeTraceforObjects(Sphere)
  (params (DegreesPerTrace :type Float%20%28single-precision%29) (NumberOfTraces :type Integer) (Forward%20Vector :type Vector) (ActorLocation :type Vector) (ConeRadius :type Float%20%28single-precision%29) (TraceSettings :type Struct%20Trace%20Settings%20Structure))
  (for _index (range 0 NumberOfTraces)
    (bind (_outhit _returnvalue) (Collision|SphereTraceForObjects (.worldcontextobject TraceSettings) ActorLocation (+ ActorLocation (* (Math|Vector|RotateVector (Math|Vector|RotateVector Forward%20Vector (Math|Rotator|MakeRotator 0.0 0.0 (/ (* NumberOfTraces DegreesPerTrace) -2.0))) (Math|Rotator|MakeRotator 0.0 0.0 (* _index DegreesPerTrace))) ConeRadius)) (.radius TraceSettings) (.objecttypes TraceSettings) (.tracecomplex TraceSettings) (.actorstoignore TraceSettings) (.drawdebugtype TraceSettings) (.ignoreself TraceSettings) (.tracecolour TraceSettings) (.tracehitcolour TraceSettings) (.drawtime TraceSettings)))
    (if _returnvalue
      (Utilities|Array|AddUnique (LocalVariables|GetActorsInCone) (.hitactor _outhit))))
  (return (LocalVariables|GetActorsInCone)))

(fn PlaceatHeightOfCapsule
  (params (ActorLocation :type Vector) (CapsuleCollider :type Capsule%20Component%20Object%20Reference) (Selection :type String))
  (switch string Selection
    (:Top
      (return (+ ActorLocation (Math|Vector|MakeVector 0.0 0.0 (+ (Components|Capsule|GetScaledCapsuleHalfHeight CapsuleCollider) 3.5)))))
    (:Bottom
      (return (- ActorLocation (Math|Vector|MakeVector 0.0 0.0 (- (Components|Capsule|GetScaledCapsuleHalfHeight CapsuleCollider) 3.5)))))))

(fn CheckIsArrayEmpty(Actors)
  (params (Actors :type Array%20of%20Actor%20Object%20References))
  (return (== (Utilities|Array|Length Actors) 0)))

(fn AngleBetweenVectors
  (params (First%20Vector :type Vector) (Second%20Vector :type Vector))
  (return (Class|KismetMathLibrary|DegAcos (Math|Vector|DotProduct (Math|Vector|Normalize First%20Vector) (Math|Vector|Normalize Second%20Vector)))))

(fn HasMatchingTags
  (params (Target :type Object%20Object%20Reference) (Tags :type Gameplay%20Tag%20Container%20Structure))
  (bind _tags_container (Class|ALSGameplayTagsBPI|BPIGetTags(Message) Target))
  (Utilities|Array|ForEachLoopwithBreak (GameplayTags|BreakGameplayTagContainer _tags_container)
    (:LoopBody
      (if (GameplayTags|HasAllTags _tags_container Tags true)
        (return true)))
    (:Completed
      (return false))))

(fn HasMatchingTag(Pure)
  (params (Target :type Object%20Object%20Reference) (Tags :type Gameplay%20Tag%20Container%20Structure))
  (bind _tags_container (Class|ALSGameplayTagsBPI|BPIGetTags(Message) Target))
  (Utilities|Array|ForEachLoopwithBreak (GameplayTags|BreakGameplayTagContainer _tags_container)
    (:LoopBody
      (if (GameplayTags|HasAllTags _tags_container Tags true)
        (return true)))
    (:Completed
      (return false))))