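; Blueprint function library that wraps data table lookups for freeflow combat and trace positions.
; GetWeaponTypeRow reads a weapon type's row from FreeflowCombatTable, and RetrieveTracePostionData reads a row from DT_TracePostions.
; GetRandomSpecialAttack uses the weapon row to return attacker and victim special combo animations.
; Each animation uses its own random index call, both bounded by the attacker array's length, so the pair can mismatch.
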(fn GetWeaponTypeRow
  (params (RowName :type Name))
  (bind _output_get (LocalVariables|SetRow%20Name RowName))
  (bind _returnvalue (Utilities|GetDataTableRow "/Game/Revenant/_Core/Combat/DataTables/FreeflowCombatTable.FreeflowCombatTable" _output_get)
    (:then
      (return _returnvalue))))

(fn RetrieveTracePostionData
  (params (Row%20Name :type String))
  (bind _returnvalue (Utilities|GetDataTableRow "/Game/Revenant/_Core/Combat/DataTables/DT_TracePostions.DT_TracePostions" (Utilities|String|StringToName Row%20Name))
    (:then
      (return _returnvalue))))

(fn GetRandomSpecialAttack
  (params (RowName :type Name))
  (bind _combatweaponanimationsstruct (CallFunction|GetWeaponTypeRow RowName))
  (return (Utilities|Array|Get(acopy) (.attacker (.specialcombomoves _combatweaponanimationsstruct)) (Math|Random|RandomIntegerinRange 0 (- (Utilities|Array|Length (.attacker (.specialcombomoves _combatweaponanimationsstruct))) 1))) (Utilities|Array|Get(acopy) (.victim (.specialcombomoves _combatweaponanimationsstruct)) (Math|Random|RandomIntegerinRange 0 (- (Utilities|Array|Length (.attacker (.specialcombomoves _combatweaponanimationsstruct))) 1)))))