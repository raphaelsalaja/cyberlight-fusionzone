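; BP_Weapon is a weapon actor with a configurable static mesh and two particle trail effects, a main trail and dust.
; On BeginPlay it applies the trail and dust templates to their particle components and assigns the desired mesh.
; StartTrails and EndTrails switch both anim-trail emitters on and off, stretching them between the mesh's Start and End sockets with a centred width.
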(event EventBeginPlay
  (CallFunction|SetTemplates)
  (CallFunction|SetMesh))

(fn ConstructionScript)

(fn SetTemplates
  (Effects|Components|ParticleSystem|SetTemplate (Variables|Default|GetTrail) (Variables|Default|GetTrailTemplate))
  (Effects|Components|ParticleSystem|SetTemplate (Variables|Default|GetDust) (Variables|Default|GetDustTemplate))
  (return))

(fn StartTrails
  (Utilities|FlowControl|Sequence
    (:then_0
      (bind _trail (Variables|Default|GetTrail)
        (:then
          (Effects|Particles|Trails|BeginTrails _trail "Start" "End" "ETrailWidthMode_FromCentre" 1.0))
        (:else)))
    (:then_1
      (bind _dust (Variables|Default|GetDust)
        (:then
          (Effects|Particles|Trails|BeginTrails _dust "Start" "End" "ETrailWidthMode_FromCentre" 1.0))
        (:else)))))

(fn EndTrails
  (Utilities|FlowControl|Sequence
    (:then_0
      (bind _trail (Variables|Default|GetTrail)
        (:then
          (Effects|Particles|Trails|EndTrails _trail))
        (:else)))
    (:then_1
      (bind _dust (Variables|Default|GetDust)
        (:then
          (Effects|Particles|Trails|EndTrails _dust))
        (:else)))))

(fn SetMesh
  (Components|StaticMesh|SetStaticMesh (Variables|Default|GetStaticMesh) (Variables|Default|GetDesiredStaticMesh)))