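; Animation modifier that builds combat notify tracks on an attack animation, replacing all existing notify tracks when applied.
; It splits the clip into equal intervals by attack count, each getting its own Attack Window track with a trace window state whose position comes from the Attacks array.
; Each interval also starts with a whoosh sound on an Audio track, and a trail state spans the whole clip on a Particle Effects track.
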(event EventOnApply
  (params (AnimationSequence :type Anim%20Sequence%20Object%20Reference))
  ;[0 0 0] Add Animation Modifier
  (Variables|Default|SetAnimSequence AnimationSequence)
  (Utilities|FlowControl|Sequence
    (:then_0
      (Class|AnimationBlueprintLibrary|RemoveAllAnimationNotifyTracks (Variables|Default|GetAnimSequence)))
    (:then_1
      (CallFunction|CreateTrackSlots))))

(fn CreateTrackSlots
  (bind _animsequence (Variables|Default|GetAnimSequence))
  (Utilities|FlowControl|Sequence
    (:then_0
      (Class|AnimationBlueprintLibrary|AddAnimationNotifyTrack (Variables|Default|GetAnimSequence) "Audio" "(R=1.000000,G=0.000000,B=0.000000,A=1.000000)")
      (Class|AnimationBlueprintLibrary|AddAnimationNotifyTrack (Variables|Default|GetAnimSequence) "Particle Effects" "(R=1.000000,G=0.000000,B=0.000000,A=1.000000)"))
    (:then_1
      (for _index (range 1 (Variables|Default|GetAttackAmount))
        (LocalVariables|SetTrackName (Utilities|String|StringToName (Utilities|String|BuildString(Integer) "Attack Window " "" _index)))
        (Utilities|FlowControl|Sequence
          (:then_0
            (Class|AnimationBlueprintLibrary|AddAnimationNotifyTrack (Variables|Default|GetAnimSequence) (LocalVariables|GetTrackName) "(R=1.000000,G=0.000000,B=0.000000,A=1.000000)")
            (bind _returnvalue (Class|AnimationBlueprintLibrary|AddAnimationNotifyEvent (Variables|Default|GetAnimSequence) "Audio" (LocalVariables|GetStartTime) "/Game/Revenant/Blueprints/AnimationNotifiers/AN_PlaySound.AN_PlaySound_C"))
            (bind _asan_play_sound (Utilities|Casting|CastToAN_PlaySound _returnvalue))
            (Variables|/Game/Revenant/Blueprints/AnimationNotifiers/AN_PlaySound.AN_PlaySound_C|SetSound _asan_play_sound "/Game/Revenant/Audio/Combat/BareHands/Wavs/SuperShortTransitionWhooshA.SuperShortTransitionWhooshA"))
          (:then_1
            (bind _returnvalue_2 (Class|AnimationBlueprintLibrary|AddAnimationNotifyStateEvent (Variables|Default|GetAnimSequence) (LocalVariables|GetTrackName) (LocalVariables|GetStartTime) (CallFunction|CalculateIntervals) "/Game/Revenant/Blueprints/AnimationNotifiers/ANS_TraceWindow.ANS_TraceWindow_C"))
            (bind _asans_trace_window (Utilities|Casting|CastToANS_TraceWindow _returnvalue_2))
            (Variables|/Game/Revenant/Blueprints/AnimationNotifiers/ANS_TraceWindow.ANS_TraceWindow_C|SetTracePosition _asans_trace_window (select (Utilities|Array|IsValidIndex (Variables|Default|GetAttacks) (- _index 1)) (Utilities|Array|Get(acopy) (Variables|Default|GetAttacks) (- _index 1)) "NewEnumerator0"))
            (LocalVariables|SetStartTime (+ (LocalVariables|GetStartTime) (CallFunction|CalculateIntervals)))))))
    (:then_2
      (Class|AnimationBlueprintLibrary|AddAnimationNotifyStateEvent _animsequence "Particle Effects" 0.0 (Class|AnimationBlueprintLibrary|GetSequenceLength _animsequence) "/Game/Revenant/Blueprints/AnimationNotifiers/ANS_Trail.ANS_Trail_C"))))

(fn CleanUpAnimation)

(fn InsertAnimationModifiers)

(fn CalculateIntervals
  (return (/ (Animation|GetPlayLength (Variables|Default|GetAnimSequence)) (Variables|Default|GetAttackAmount))))