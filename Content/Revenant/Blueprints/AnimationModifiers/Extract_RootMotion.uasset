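; Animation Modifier that bakes an animation sequence's root bone translation into float curves.
; On apply it wipes all existing curve data, adds the curves in CurveNames, keys RootMotion_Factor once at 1 and writes RootMotion_X, Y and Z every frame.
; Revert removes the listed curves but keeps their names on the skeleton, without restoring wiped data.
; A root yaw key node exists but is never run.
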(event EventOnRevert
  (params (AnimationSequence :type Anim%20Sequence%20Object%20Reference))
  (Variables|Default|SetAnimation%20Sequence AnimationSequence)
  (for _array_element (Variables|Default|GetCurve%20Names)
    (Class|AnimationBlueprintLibrary|RemoveCurve (Variables|Default|GetAnimation%20Sequence) _array_element false)))

(event EventOnApply
  (params (AnimationSequence :type Anim%20Sequence%20Object%20Reference))
  (bind _output_get (Variables|Default|SetAnimation%20Sequence AnimationSequence))
  (Class|AnimationBlueprintLibrary|RemoveAllCurveData _output_get)
  (for _array_element (Variables|Default|GetCurve%20Names)
    (Class|AnimationBlueprintLibrary|AddCurve (Variables|Default|GetAnimation%20Sequence) _array_element "RCT_Float" false))
  (Class|AnimationBlueprintLibrary|AddFloatCurveKey (Variables|Default|GetAnimation%20Sequence) "RootMotion_Factor" 0.0 1.0)
  (for _index (range 0 (- (Class|AnimationBlueprintLibrary|GetNumFrames (Variables|Default|GetAnimation%20Sequence)) 1))
    (Class|AnimationBlueprintLibrary|AddFloatCurveKey (Variables|Default|GetAnimation%20Sequence) "RootMotion_X" (Class|AnimationBlueprintLibrary|GetTimeatFrame (Variables|Default|GetAnimation%20Sequence) _index) (.x (.location (Class|AnimationBlueprintLibrary|GetBonePoseforFrame (Variables|Default|GetAnimation%20Sequence) "root" _index false))))
    (Class|AnimationBlueprintLibrary|AddFloatCurveKey (Variables|Default|GetAnimation%20Sequence) "RootMotion_Y" (Class|AnimationBlueprintLibrary|GetTimeatFrame (Variables|Default|GetAnimation%20Sequence) _index) (.y (.location (Class|AnimationBlueprintLibrary|GetBonePoseforFrame (Variables|Default|GetAnimation%20Sequence) "root" _index false))))
    (Class|AnimationBlueprintLibrary|AddFloatCurveKey (Variables|Default|GetAnimation%20Sequence) "RootMotion_Z" (Class|AnimationBlueprintLibrary|GetTimeatFrame (Variables|Default|GetAnimation%20Sequence) _index) (.z (.location (Class|AnimationBlueprintLibrary|GetBonePoseforFrame (Variables|Default|GetAnimation%20Sequence) "root" _index false))))))