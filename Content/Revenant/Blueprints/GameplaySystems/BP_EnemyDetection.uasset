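; Enemy detection component that uses an EQS query to pick a single enemy actor for its owner, the player.
; RunEnemyDetectionQuery first checks the owner's gameplay tags through an interface message, printing the reason when the player is attacking.
; EnemyDetectionProcessing stores a successful result as DetectedEnemy.
; Any other query status appends the Combat.Enable.Detections tag to the owner.
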(event EventBeginPlay
  (Events|BeginPlayInitialization))

(fn RunEnemyDetectionQuery
  (bind (_result _reason) (Checks|CheckifAbletoRunQuery))
  (if _result
    (bind _returnvalue (AI|EQS|RunEQSQuery "/Game/Revenant/Blueprints/EnviromentQuerySystems/Combat/EQS_EnemyDetection.EQS_EnemyDetection" (Components|GetOwner) "SingleResult"))
    (EventDispatchers|BindEventtoOnQueryFinishedEvent _returnvalue (EventDispatchers|CreateEvent :!event EnemyDetectionProcessing))
    (else
      (Debug|PrintFailureReason true false "(R=0.000000,G=0.000000,B=0.000000,A=1.000000)" 0.0 "Cannot Run The Query 
Reason: " _reason))))

(fn CheckifAbletoRunQuery
  (Utilities|FlowControl|Sequence
    (:then_0
      (bind _tags_container (Class|ALSGameplayTagsBPI|BPIGetTags(Message) (Variables|Default|GetOwner)))
      (if (GameplayTags|HasTag :TagContainer _tags_container)
        (return false "The Player is Currently Attacking")))))

(fn PrintFailureReason
  (params (bPrintToScreen :type Boolean) (bPrintToLog :type Boolean) (TextColor :type Linear%20Color%20Structure) (Duration :type Float%20%28single-precision%29) (Prefix :type String) (Reason :type String))
  (Development|PrintString (Utilities|String|Append Prefix Reason) bPrintToScreen bPrintToLog TextColor Duration))

(fn EnemyDetectionProcessing
  (params (QueryInstance :type Env%20Query%20Instance%20Blueprint%20Wrapper%20Object%20Reference) (QueryStatus :type EEnvQueryStatus%20Enum :default "Processing"))
  (switch Utilities|FlowControl|Switch|SwitchonEEnvQueryStatus QueryStatus
    (:Processing
      (Class|ALSGameplayTagsBPI|BPIAppendTags(Message) (Variables|Default|GetOwner) "(GameplayTags=((TagName=\"Combat.Enable.Detections\")))" :!label _label))
    (:Success
      (bind _resultactors (AI|EQS|GetQueryResultsasActors QueryInstance))
      (Variables|Default|SetDetected%20Enemy (Utilities|Array|Get(acopy) _resultactors)))
    (:Failed
      (goto _label))
    (:Aborted
      (goto _label))
    (:OwnerLost
      (goto _label))
    (:MissingParam
      (goto _label))))

(fn BeginPlayInitialization
  (Variables|Default|SetOwner (Components|GetOwner)))